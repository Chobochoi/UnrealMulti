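; Rubik's Cube-style actor with clockwise and counterclockwise turn events for the Up, Down, Front, Back, Right and Left faces.
; After a short delay, each event fans line traces around that face's center cube and attaches hit components to it, keeping world transforms.
; A per-event timeline then lerps the center cube 90 degrees on one axis, carrying the attached pieces.
; All faces share one accumulated angle, FloatRotValue, updated when each timeline finishes.
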(event Custom|RUEvent
  (bind _last_index (Variables|Default|GetLast%20Index))
  ;[1 1 1] U/RU Event
  (Utilities|FlowControl|Delay 0.1)
  (for _index (range 0 _last_index)
    (CallFunction|MakeLineTrace (Variables|Default|GetUpCube) 0.0 0.0 (* _index (CallFunction|HowManyLine _last_index))))
  (bind (_acentercube _rotator) (CallFunction|GoRotate (Variables|Default|GetUpCube)))
  (bind _새_트랙_0 (Timeline|타임라인_1 PlayFromStart)
    (:Update
      (Variables|Default|SetReturnRotValue (Math|Float|Lerp (Variables|Default|GetFloatRotValue) (+ (Variables|Default|GetFloatRotValue) -9e+01) _새_트랙_0))
      (Transformation|SetRelativeRotation _acentercube (Math|Rotator|MakeRotator 0.0 0.0 (Math|Float|Lerp (Variables|Default|GetFloatRotValue) (+ (Variables|Default|GetFloatRotValue) -9e+01) _새_트랙_0)) false false))
    (:Finished
      (Variables|Default|SetFloatRotValue (Variables|Default|GetReturnRotValue)))))

(event Custom|RREvent
  (bind _last_index (Variables|Default|GetLast%20Index))
  (bind _rightcube (Variables|Default|GetRightCube))
  ;[1 1 1] R/RR Event
  (Utilities|FlowControl|Delay 0.1)
  (for _index (range 0 _last_index)
    (CallFunction|NewFunction0 (* _index (CallFunction|HowManyLine _last_index)) 0.0 0.0 _rightcube))
  (bind (_acentercube _rotator) (CallFunction|GoRotate _rightcube))
  (bind _새_트랙_0 (Timeline|타임라인_9 PlayFromStart)
    (:Update
      (Variables|Default|SetReturnRotValue (Math|Float|Lerp (Variables|Default|GetFloatRotValue) (+ (Variables|Default|GetFloatRotValue) -9e+01) _새_트랙_0))
      (Transformation|SetRelativeRotation _acentercube (Math|Rotator|MakeRotator (Math|Float|Lerp (Variables|Default|GetFloatRotValue) (+ (Variables|Default|GetFloatRotValue) -9e+01) _새_트랙_0) 0.0 0.0) false false))
    (:Finished
      (Variables|Default|SetFloatRotValue (Variables|Default|GetReturnRotValue)))))

(event Custom|BEvent
  (bind _last_index (Variables|Default|GetLast%20Index))
  (bind _backcube (Variables|Default|GetBackCube))
  ;[1 1 1] B/RB Event
  (Utilities|FlowControl|Delay 0.1)
  (for _index (range 0 _last_index)
    (CallFunction|MakeLineTrace _backcube 0.0 (* _index (CallFunction|HowManyLine _last_index)) 0.0))
  (bind (_acentercube _rotator) (CallFunction|GoRotate _backcube))
  (bind _새_트랙_0 (Timeline|타임라인_6 PlayFromStart)
    (:Update
      (Variables|Default|SetReturnRotValue (Math|Float|Lerp (Variables|Default|GetFloatRotValue) (+ (Variables|Default|GetFloatRotValue) 9e+01) _새_트랙_0))
      (Transformation|SetRelativeRotation _acentercube (Math|Rotator|MakeRotator 0.0 (Math|Float|Lerp (Variables|Default|GetFloatRotValue) (+ (Variables|Default|GetFloatRotValue) 9e+01) _새_트랙_0) 0.0) false false))
    (:Finished
      (Variables|Default|SetFloatRotValue (Variables|Default|GetReturnRotValue)))))

(event Custom|RLEvent
  (bind _last_index (Variables|Default|GetLast%20Index))
  (bind _floatrotvalue (Variables|Default|GetFloatRotValue))
  (bind _leftcube (Variables|Default|GetLeftCube))
  ;[1 1 1] L/RL Event
  (Utilities|FlowControl|Delay 0.1)
  (for _index (range 0 _last_index)
    (CallFunction|NewFunction0 (* _index (CallFunction|HowManyLine _last_index)) 0.0 0.0 _leftcube))
  (bind (_acentercube _rotator) (CallFunction|GoRotate _leftcube))
  (bind _새_트랙_0 (Timeline|타임라인_11 PlayFromStart)
    (:Update
      (Variables|Default|SetReturnRotValue (Math|Float|Lerp _floatrotvalue (+ _floatrotvalue -9e+01) _새_트랙_0))
      (Transformation|SetRelativeRotation _acentercube (Math|Rotator|MakeRotator (Math|Float|Lerp _floatrotvalue (+ _floatrotvalue -9e+01) _새_트랙_0) 0.0 0.0) false false))))

(event Custom|REvent
  (bind _last_index (Variables|Default|GetLast%20Index))
  (bind _rightcube (Variables|Default|GetRightCube))
  ;[1 1 1] R/RR Event
  (Utilities|FlowControl|Delay 0.1)
  (for _index (range 0 _last_index)
    (CallFunction|NewFunction0 (* _index (CallFunction|HowManyLine _last_index)) 0.0 0.0 _rightcube))
  (bind (_acentercube _rotator) (CallFunction|GoRotate _rightcube))
  (bind _새_트랙_0 (Timeline|타임라인_8 PlayFromStart)
    (:Update
      (Variables|Default|SetReturnRotValue (Math|Float|Lerp (Variables|Default|GetFloatRotValue) (+ (Variables|Default|GetFloatRotValue) 9e+01) _새_트랙_0))
      (Transformation|SetRelativeRotation _acentercube (Math|Rotator|MakeRotator (Math|Float|Lerp (Variables|Default|GetFloatRotValue) (+ (Variables|Default|GetFloatRotValue) 9e+01) _새_트랙_0) 0.0 0.0) false false))
    (:Finished
      (Variables|Default|SetFloatRotValue (Variables|Default|GetReturnRotValue)))))

(event Custom|LEvent
  (bind _last_index (Variables|Default|GetLast%20Index))
  (bind _leftcube (Variables|Default|GetLeftCube))
  ;[1 1 1] L/RL Event
  (Utilities|FlowControl|Delay 0.1)
  (for _index (range 0 _last_index)
    (CallFunction|NewFunction0 (* _index (CallFunction|HowManyLine _last_index)) 0.0 0.0 _leftcube))
  (bind (_acentercube _rotator) (CallFunction|GoRotate _leftcube))
  (bind _새_트랙_0 (Timeline|타임라인_10 PlayFromStart)
    (:Update
      (Variables|Default|SetReturnRotValue (Math|Float|Lerp (Variables|Default|GetFloatRotValue) (+ (Variables|Default|GetFloatRotValue) 9e+01) _새_트랙_0))
      (Transformation|SetRelativeRotation _acentercube (Math|Rotator|MakeRotator (Math|Float|Lerp (Variables|Default|GetFloatRotValue) (+ (Variables|Default|GetFloatRotValue) 9e+01) _새_트랙_0) 0.0 0.0) false false))
    (:Finished
      (Variables|Default|SetFloatRotValue (Variables|Default|GetReturnRotValue)))))

(event Custom|FEvent
  (bind _last_index (Variables|Default|GetLast%20Index))
  (bind _frontcube (Variables|Default|GetFrontCube))
  ;[1 1 1] F/RF Event
  (Utilities|FlowControl|Delay 0.1)
  (for _index (range 0 _last_index)
    (CallFunction|MakeLineTrace _frontcube 0.0 (* _index (CallFunction|HowManyLine _last_index)) 0.0))
  (bind (_acentercube _rotator) (CallFunction|GoRotate _frontcube))
  (bind _새_트랙_0 (Timeline|타임라인_4 PlayFromStart)
    (:Update
      (Variables|Default|SetReturnRotValue (Math|Float|Lerp (Variables|Default|GetFloatRotValue) (+ (Variables|Default|GetFloatRotValue) 9e+01) _새_트랙_0))
      (Transformation|SetRelativeRotation _frontcube (Math|Rotator|MakeRotator 0.0 (Math|Float|Lerp (Variables|Default|GetFloatRotValue) (+ (Variables|Default|GetFloatRotValue) 9e+01) _새_트랙_0) 0.0) false false))
    (:Finished
      (Variables|Default|SetFloatRotValue (Variables|Default|GetReturnRotValue)))))

(event Custom|RFEvent
  (bind _last_index (Variables|Default|GetLast%20Index))
  (bind _frontcube (Variables|Default|GetFrontCube))
  ;[1 1 1] F/RF Event
  (Utilities|FlowControl|Delay 0.1)
  (for _index (range 0 _last_index)
    (CallFunction|MakeLineTrace _frontcube 0.0 (* _index (CallFunction|HowManyLine _last_index)) 0.0))
  (bind (_acentercube _rotator) (CallFunction|GoRotate _frontcube))
  (bind _새_트랙_0 (Timeline|타임라인_5 PlayFromStart)
    (:Update
      (Variables|Default|SetReturnRotValue (Math|Float|Lerp (Variables|Default|GetFloatRotValue) (+ (Variables|Default|GetFloatRotValue) -9e+01) _새_트랙_0))
      (Transformation|SetRelativeRotation _acentercube (Math|Rotator|MakeRotator 0.0 (Math|Float|Lerp (Variables|Default|GetFloatRotValue) (+ (Variables|Default|GetFloatRotValue) -9e+01) _새_트랙_0) 0.0) false false))
    (:Finished
      (Variables|Default|SetFloatRotValue (Variables|Default|GetReturnRotValue)))))

(event Custom|Devent
  (bind _last_index (Variables|Default|GetLast%20Index))
  ;[1 1 1] D/RD Event
  (Utilities|FlowControl|Delay 0.1)
  (for _index (range 0 _last_index)
    (CallFunction|MakeLineTrace (Variables|Default|GetDownCube) 0.0 0.0 (* _index (CallFunction|HowManyLine _last_index))))
  (bind (_acentercube _rotator) (CallFunction|GoRotate (Variables|Default|GetDownCube)))
  (bind _새_트랙_0 (Timeline|타임라인_2 PlayFromStart)
    (:Update
      (Variables|Default|SetReturnRotValue (Math|Float|Lerp (Variables|Default|GetFloatRotValue) (+ (Variables|Default|GetFloatRotValue) 9e+01) _새_트랙_0))
      (Transformation|SetRelativeRotation _acentercube (Math|Rotator|MakeRotator 0.0 0.0 (Math|Float|Lerp (Variables|Default|GetFloatRotValue) (+ (Variables|Default|GetFloatRotValue) 9e+01) _새_트랙_0)) false false))
    (:Finished
      (Variables|Default|SetFloatRotValue (Variables|Default|GetReturnRotValue)))))

(event Custom|RDEvent
  (bind _last_index (Variables|Default|GetLast%20Index))
  ;[1 1 1] D/RD Event
  (Utilities|FlowControl|Delay 0.1)
  (for _index (range 0 _last_index)
    (CallFunction|MakeLineTrace (Variables|Default|GetDownCube) 0.0 0.0 (* _index (CallFunction|HowManyLine _last_index))))
  (bind (_acentercube _rotator) (CallFunction|GoRotate (Variables|Default|GetDownCube)))
  (bind _새_트랙_0 (Timeline|타임라인_3 PlayFromStart)
    (:Update
      (Variables|Default|SetReturnRotValue (Math|Float|Lerp (Variables|Default|GetFloatRotValue) (+ (Variables|Default|GetFloatRotValue) -9e+01) _새_트랙_0))
      (Transformation|SetRelativeRotation _acentercube (Math|Rotator|MakeRotator 0.0 0.0 (Math|Float|Lerp (Variables|Default|GetFloatRotValue) (+ (Variables|Default|GetFloatRotValue) -9e+01) _새_트랙_0)) false false))
    (:Finished
      (Variables|Default|SetFloatRotValue (Variables|Default|GetReturnRotValue)))))

(event Custom|UEvent
  (bind _last_index (Variables|Default|GetLast%20Index))
  ;[1 1 1] U/RU Event
  (Utilities|FlowControl|Delay 0.1)
  (for _index (range 0 _last_index)
    (CallFunction|MakeLineTrace (Variables|Default|GetUpCube) 0.0 0.0 (* _index (CallFunction|HowManyLine _last_index))))
  (bind (_acentercube _rotator) (CallFunction|GoRotate (Variables|Default|GetUpCube)))
  (bind _새_트랙_0 (Timeline|타임라인_0 PlayFromStart)
    (:Update
      (Variables|Default|SetReturnRotValue (Math|Float|Lerp (Variables|Default|GetFloatRotValue) (+ (Variables|Default|GetFloatRotValue) 9e+01) _새_트랙_0))
      (Transformation|SetRelativeRotation _acentercube (Math|Rotator|MakeRotator 0.0 0.0 (Math|Float|Lerp (Variables|Default|GetFloatRotValue) (+ (Variables|Default|GetFloatRotValue) 9e+01) _새_트랙_0)) false false))
    (:Finished
      (Variables|Default|SetFloatRotValue (Variables|Default|GetReturnRotValue)))))

(event Custom|RBEvent
  (bind _last_index (Variables|Default|GetLast%20Index))
  (bind _backcube (Variables|Default|GetBackCube))
  ;[1 1 1] B/RB Event
  (Utilities|FlowControl|Delay 0.1)
  (for _index (range 0 _last_index)
    (CallFunction|MakeLineTrace _backcube 0.0 (* _index (CallFunction|HowManyLine _last_index)) 0.0))
  (bind (_acentercube _rotator) (CallFunction|GoRotate _backcube))
  (bind _새_트랙_0 (Timeline|타임라인_7 PlayFromStart)
    (:Update
      (Variables|Default|SetReturnRotValue (Math|Float|Lerp (Variables|Default|GetFloatRotValue) (+ (Variables|Default|GetFloatRotValue) -9e+01) _새_트랙_0))
      (Transformation|SetRelativeRotation _acentercube (Math|Rotator|MakeRotator 0.0 (Math|Float|Lerp (Variables|Default|GetFloatRotValue) (+ (Variables|Default|GetFloatRotValue) -9e+01) _새_트랙_0) 0.0) false false))
    (:Finished
      (Variables|Default|SetFloatRotValue (Variables|Default|GetReturnRotValue)))))

(fn ConstructionScript)

(fn MakeLineTrace
  (params (CenterCube :type Static%20Mesh%20Component%20Object%20Reference) (x :type Float%20%28single-precision%29) (y :type Float%20%28single-precision%29) (z :type Float%20%28single-precision%29))
  (bind _returnvalue (Transformation|GetWorldLocation CenterCube))
  (bind _outhit (Collision|LineTraceForObjects _returnvalue (+ _returnvalue (* (Math|Vector|RotateVector (Math|Vector|GetForwardVector CenterCube) (Math|Rotator|MakeRotator x y z)) (Variables|Default|GetDistance))) (Utilities|Array|MakeArray "ObjectTypeQuery2") false 0 "None" false))
  (Transformation|AttachComponentToComponent (.HitComponent (Collision|BreakHitResult _outhit)) CenterCube "None" "KeepWorld" "KeepWorld" "KeepRelative" true))

(fn HowManyLine
  (params (NewParam :type Integer))
  (return (/ 3.6e+02 (Math|Conversions|ToFloat(Integer) (+ NewParam 1)))))

(fn GoRotate
  (params (CenterCube :type Static%20Mesh%20Component%20Object%20Reference))
  (bind _output_get (Variables|Default|SetRelative%20Rotation (Variables|/Script/Engine.SceneComponent|GetRelativeRotation CenterCube)))
  (return CenterCube (Math|Rotator|MakeRotator (.Roll (Math|Rotator|BreakRotator _output_get)) (.Pitch (Math|Rotator|BreakRotator _output_get)) (.Yaw (Math|Rotator|BreakRotator _output_get)))))

(fn LerpValue
  (params (Alpha :type Float%20%28single-precision%29) (CenterCube :type Static%20Mesh%20Component%20Object%20Reference) (NewParam :type Rotator))
  (bind _output_get (Variables|Default|SetRelative%20Rotation (Variables|/Script/Engine.SceneComponent|GetRelativeRotation CenterCube)))
  (return (Math|Rotator|Lerp(Rotator) _output_get "0, 0, 0" Alpha true)))

(fn NewFunction0
  (params (NewParam :type Float%20%28single-precision%29) (NewParam1 :type Float%20%28single-precision%29) (NewParam2 :type Float%20%28single-precision%29) (NewParam3 :type Static%20Mesh%20Component%20Object%20Reference))
  (bind _returnvalue (Transformation|GetWorldLocation NewParam3))
  (bind _outhit (Collision|LineTraceForObjects _returnvalue (+ _returnvalue (* (Math|Vector|RotateVector (Math|Vector|GetUpVector NewParam3) (Math|Rotator|MakeRotator NewParam NewParam1 NewParam2)) (Variables|Default|GetDistance))) (Utilities|Array|MakeArray "ObjectTypeQuery2") false 0 "None" false))
  (Transformation|AttachComponentToComponent (.HitComponent (Collision|BreakHitResult _outhit)) NewParam3 "None" "KeepWorld" "KeepWorld" "KeepRelative" true))