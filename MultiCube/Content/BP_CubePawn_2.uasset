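; Player pawn for a Rubik's-style cube puzzle, turning keyboard input into face moves on the level's BP_RealCubeActor.
; U, D, F, B, R, L keys and their Reverse input actions call cube events, while Space fires one random move.
; It creates BP_MultiUI, highlights pressed keys and swaps normal/reverse panels on Shift.
; Mouse axes drive control rotation, left click hides the cursor while held, and P shows the exit panel.
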(event EventBeginPlay
  (bind _returnvalue (UserInterface|CreateWidget "/Game/BP_MultiUI.BP_MultiUI_C"))
  (bind _output_get (Variables|Default|SetMultiUI _returnvalue))
  (bind _outactors (Actor|GetAllActorsOfClass "/Game/BP_RealCubeActor.BP_RealCubeActor_C"))
  (Variables|Default|SetRealCube (Utilities|Array|Get(acopy) _outactors))
  (UserInterface|Viewport|AddtoViewport _output_get 0))

(event Input|ActionEvents|InputActionReverseU
  (params (Key :type Key%20Structure :default "None"))
  (bind _multiui (Variables|Default|GetMultiUI))
  (bind _utext (Variables|/Game/BP_MultiUI.BP_MultiUI_C|GetUText _multiui))
  (:Pressed
    (Default|RUEvent (Variables|Default|GetRealCube))
    (Appearance|SetColorandOpacity _utext (Variables|Default|GetText%20Green) :!class /Script/UMG.TextBlock))
  (:Released
    (Appearance|SetColorandOpacity _utext (Variables|Default|GetText%20Orign) :!class /Script/UMG.TextBlock)))

(event Input|ActionEvents|InputActionReverseD
  (params (Key :type Key%20Structure :default "None"))
  (bind _multiui (Variables|Default|GetMultiUI))
  (:Pressed
    (Default|RDEvent (Variables|Default|GetRealCube))
    (Appearance|SetColorandOpacity (Variables|/Game/BP_MultiUI.BP_MultiUI_C|GetDText _multiui) (Variables|Default|GetText%20Green) :!class /Script/UMG.TextBlock))
  (:Released
    (Appearance|SetColorandOpacity (Variables|/Game/BP_MultiUI.BP_MultiUI_C|GetRDText _multiui) (Variables|Default|GetText%20Orign) :!class /Script/UMG.TextBlock)))

(event Input|ActionEvents|InputActionReverseF
  (params (Key :type Key%20Structure :default "None"))
  (bind _multiui (Variables|Default|GetMultiUI))
  (bind _ftext (Variables|/Game/BP_MultiUI.BP_MultiUI_C|GetFText _multiui))
  (:Pressed
    (Default|RFEvent (Variables|Default|GetRealCube))
    (Appearance|SetColorandOpacity _ftext (Variables|Default|GetText%20Green) :!class /Script/UMG.TextBlock))
  (:Released
    (Appearance|SetColorandOpacity _ftext (Variables|Default|GetText%20Orign) :!class /Script/UMG.TextBlock)))

(event Input|ActionEvents|InputActionReverseB
  (params (Key :type Key%20Structure :default "None"))
  (bind _multiui (Variables|Default|GetMultiUI))
  (bind _btext (Variables|/Game/BP_MultiUI.BP_MultiUI_C|GetBText _multiui))
  (:Pressed
    (Default|RBEvent (Variables|Default|GetRealCube))
    (Appearance|SetColorandOpacity _btext (Variables|Default|GetText%20Green) :!class /Script/UMG.TextBlock))
  (:Released
    (Appearance|SetColorandOpacity _btext (Variables|Default|GetText%20Orign) :!class /Script/UMG.TextBlock)))

(event Input|ActionEvents|InputActionReverseR
  (params (Key :type Key%20Structure :default "None"))
  (bind _multiui (Variables|Default|GetMultiUI))
  (bind _rtext (Variables|/Game/BP_MultiUI.BP_MultiUI_C|GetRText _multiui))
  (:Pressed
    (Default|RREvent (Variables|Default|GetRealCube))
    (Appearance|SetColorandOpacity _rtext (Variables|Default|GetText%20Green) :!class /Script/UMG.TextBlock))
  (:Released
    (Appearance|SetColorandOpacity _rtext (Variables|Default|GetText%20Orign) :!class /Script/UMG.TextBlock)))

(event Input|ActionEvents|InputActionReverseL
  (params (Key :type Key%20Structure :default "None"))
  (bind _multiui (Variables|Default|GetMultiUI))
  (bind _ltext (Variables|/Game/BP_MultiUI.BP_MultiUI_C|GetLText _multiui))
  (:Pressed
    (Default|RLEvent (Variables|Default|GetRealCube))
    (Appearance|SetColorandOpacity _ltext (Variables|Default|GetText%20Green) :!class /Script/UMG.TextBlock))
  (:Released
    (Appearance|SetColorandOpacity _ltext (Variables|Default|GetText%20Orign) :!class /Script/UMG.TextBlock)))

(event Input|AxisEvents|InputAxisMouseX
  (params (AxisValue :type Float%20%28single-precision%29))
  (bind _returnvalue (Pawn|GetControlRotation :!class /Script/Engine.Pawn))
  ;[1 1 1] 화면 회전
  (Pawn|Input|AddControllerYawInput AxisValue)
  (Pawn|SetControlRotation (Game|GetPlayerController 0) (Math|Rotator|MakeRotator 0.0 (.pitch _returnvalue) (.yaw _returnvalue))))

(event Input|AxisEvents|InputAxisMouseY
  (params (AxisValue :type Float%20%28single-precision%29))
  ;[1 1 1] 화면 회전
  (Pawn|Input|AddControllerPitchInput AxisValue))

(event Input|KeyboardEvents|U
  (params (Key :type Key%20Structure :default "None"))
  (bind _multiui (Variables|Default|GetMultiUI))
  (bind _utext (Variables|/Game/BP_MultiUI.BP_MultiUI_C|GetUText _multiui))
  (:Pressed
    (Default|UEvent (Variables|Default|GetRealCube))
    (Appearance|SetColorandOpacity _utext (Variables|Default|GetText%20Green) :!class /Script/UMG.TextBlock))
  (:Released
    (Appearance|SetColorandOpacity _utext (Variables|Default|GetText%20Orign) :!class /Script/UMG.TextBlock)))

(event Input|KeyboardEvents|LeftShift
  (params (Key :type Key%20Structure :default "None"))
  (bind _multiui (Variables|Default|GetMultiUI))
  (bind _shifttext (Variables|/Game/BP_MultiUI.BP_MultiUI_C|GetShiftText _multiui))
  ;[1 1 1] Shift Key
  (:Pressed
    (Appearance|SetColorandOpacity _shifttext (Variables|Default|GetText%20Green) :!class /Script/UMG.TextBlock)
    (Widget|SetVisibility (Variables|/Game/BP_MultiUI.BP_MultiUI_C|GetOriginPanel (Variables|Default|GetMultiUI)) "Hidden")
    (Widget|SetVisibility (Variables|/Game/BP_MultiUI.BP_MultiUI_C|GetReversePanel (Variables|Default|GetMultiUI)) "Visible"))
  (:Released
    (Appearance|SetColorandOpacity _shifttext (Variables|Default|GetText%20Orign) :!class /Script/UMG.TextBlock)
    (Widget|SetVisibility (Variables|/Game/BP_MultiUI.BP_MultiUI_C|GetOriginPanel (Variables|Default|GetMultiUI)) "Visible")
    (Widget|SetVisibility (Variables|/Game/BP_MultiUI.BP_MultiUI_C|GetReversePanel (Variables|Default|GetMultiUI)) "Hidden")))

(event Input|KeyboardEvents|D
  (params (Key :type Key%20Structure :default "None"))
  (bind _multiui (Variables|Default|GetMultiUI))
  (:Pressed
    (Default|Devent (Variables|Default|GetRealCube))
    (Appearance|SetColorandOpacity (Variables|/Game/BP_MultiUI.BP_MultiUI_C|GetDText _multiui) (Variables|Default|GetText%20Green) :!class /Script/UMG.TextBlock))
  (:Released
    (Appearance|SetColorandOpacity (Variables|/Game/BP_MultiUI.BP_MultiUI_C|GetRDText _multiui) (Variables|Default|GetText%20Orign) :!class /Script/UMG.TextBlock)))

(event Input|KeyboardEvents|P
  (params (Key :type Key%20Structure :default "None"))
  ;[1 1 1] P 나가기
  (:Pressed
    (Variables|/Script/Engine.PlayerController|SetbShowMouseCursor (Game|GetPlayerController 0) true)
    (Widget|SetVisibility (Variables|/Game/BP_MultiUI.BP_MultiUI_C|GetExitPanel (Variables|Default|GetMultiUI)) "Visible")))

(event Input|KeyboardEvents|F
  (params (Key :type Key%20Structure :default "None"))
  (bind _multiui (Variables|Default|GetMultiUI))
  (bind _ftext (Variables|/Game/BP_MultiUI.BP_MultiUI_C|GetFText _multiui))
  (:Pressed
    (Default|FEvent (Variables|Default|GetRealCube))
    (Appearance|SetColorandOpacity _ftext (Variables|Default|GetText%20Green) :!class /Script/UMG.TextBlock))
  (:Released
    (Appearance|SetColorandOpacity _ftext (Variables|Default|GetText%20Orign) :!class /Script/UMG.TextBlock)))

(event Input|KeyboardEvents|B
  (params (Key :type Key%20Structure :default "None"))
  (bind _multiui (Variables|Default|GetMultiUI))
  (bind _btext (Variables|/Game/BP_MultiUI.BP_MultiUI_C|GetBText _multiui))
  (:Pressed
    (Default|BEvent (Variables|Default|GetRealCube))
    (Appearance|SetColorandOpacity _btext (Variables|Default|GetText%20Green) :!class /Script/UMG.TextBlock))
  (:Released
    (Appearance|SetColorandOpacity _btext (Variables|Default|GetText%20Orign) :!class /Script/UMG.TextBlock)))

(event Input|KeyboardEvents|R
  (params (Key :type Key%20Structure :default "None"))
  (bind _multiui (Variables|Default|GetMultiUI))
  (bind _rtext (Variables|/Game/BP_MultiUI.BP_MultiUI_C|GetRText _multiui))
  (:Pressed
    (Default|REvent (Variables|Default|GetRealCube))
    (Appearance|SetColorandOpacity _rtext (Variables|Default|GetText%20Green) :!class /Script/UMG.TextBlock))
  (:Released
    (Appearance|SetColorandOpacity _rtext (Variables|Default|GetText%20Orign) :!class /Script/UMG.TextBlock)))

(event Input|KeyboardEvents|L
  (params (Key :type Key%20Structure :default "None"))
  (bind _multiui (Variables|Default|GetMultiUI))
  (bind _ltext (Variables|/Game/BP_MultiUI.BP_MultiUI_C|GetLText _multiui))
  (:Pressed
    (Default|LEvent (Variables|Default|GetRealCube))
    (Appearance|SetColorandOpacity _ltext (Variables|Default|GetText%20Green) :!class /Script/UMG.TextBlock))
  (:Released
    (Appearance|SetColorandOpacity _ltext (Variables|Default|GetText%20Orign) :!class /Script/UMG.TextBlock)))

(event Input|KeyboardEvents|SpaceBar
  (params (Key :type Key%20Structure :default "None"))
  (bind _realcube (Variables|Default|GetRealCube))
  (bind _multiui (Variables|Default|GetMultiUI))
  (bind _spacetext (Variables|/Game/BP_MultiUI.BP_MultiUI_C|GetSpaceText _multiui))
  ;[1 1 1] 스페이스바
  (:Pressed
    (Appearance|SetColorandOpacity _spacetext (Variables|Default|GetText%20Green) :!class /Script/UMG.TextBlock)
    (switch int (Math|Random|RandomInteger 11)
      (:0
        (Default|UEvent _realcube))
      (:1
        (Default|RUEvent _realcube))
      (:2
        (Default|Devent _realcube))
      (:3
        (Default|RDEvent _realcube))
      (:4
        (Default|FEvent _realcube))
      (:5
        (Default|RFEvent _realcube))
      (:6
        (Default|BEvent _realcube))
      (:7
        (Default|RBEvent _realcube))
      (:8
        (Default|REvent _realcube))
      (:9
        (Default|RREvent _realcube))
      (:10
        (Default|LEvent _realcube))
      (:11
        (Default|RLEvent _realcube))))
  (:Released
    (Appearance|SetColorandOpacity _spacetext (Variables|Default|GetText%20Orign) :!class /Script/UMG.TextBlock)))

(event Input|MouseEvents|LeftMouseButton
  (params (Key :type Key%20Structure :default "None"))
  (bind _returnvalue (Game|GetPlayerController 0))
  (:Pressed
    (Variables|/Script/Engine.PlayerController|SetbShowMouseCursor _returnvalue false))
  (:Released
    (Variables|/Script/Engine.PlayerController|SetbShowMouseCursor _returnvalue true)))

(fn ConstructionScript)

(fn AddKeyArray
  (Utilities|Array|Add (Variables|Default|GetKeyValue) 0))