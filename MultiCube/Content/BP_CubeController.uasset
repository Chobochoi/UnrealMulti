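; BP_CubeController is a controller that lets the host and a client possess separate cube pawns in a networked game.
; On BeginPlay, authority caches the first BP_CubePawn and remote caches the first BP_CubePawn_2.
; M branches on authority to possess that pawn through GetPlayerController(0), with the remote path chaining ForClientPossess into ClientPossess.
; N unpossesses, while both OnRep functions are empty and the Possess event's actor lookup goes unused.
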(event Custom|For%20Client%20Possess
  (CallFunction|ClientPossess))

(event Custom|Client%20Possess
  (bind _output_get (Variables|Default|SetClientCubePawn (Variables|Default|GetClientCubePawn)))
  (Pawn|Possess (Game|GetPlayerController 0) _output_get))

(event Custom|Server%20Possess
  (bind _returnvalue (Game|GetPlayerController 0))
  (Pawn|Possess _returnvalue (Variables|Default|GetCubePawn))
  (Development|PrintString (Utilities|GetDisplayName _returnvalue)))

(event EventPossess
  (params (PossessedPawn :type Pawn%20Object%20Reference))
  (Actor|GetAllActorsOfClass (Utilities|GetClass PossessedPawn)))

(event EventBeginPlay
  (Networking|SwitchHasAuthority
    (:Authority
      (bind _outactors (Actor|GetAllActorsOfClass "/Game/BP_CubePawn.BP_CubePawn_C"))
      (Variables|Default|SetCubePawn (Utilities|Array|Get(acopy) _outactors)))
    (:Remote
      (bind _outactors_2 (Actor|GetAllActorsOfClass "/Game/BP_CubePawn_2.BP_CubePawn_2_C"))
      (Variables|Default|SetClientCubePawn (Utilities|Array|Get(acopy) _outactors_2)))))

(event Input|KeyboardEvents|N
  (params (Key :type Key%20Structure :default "None"))
  (:Pressed
    (Networking|SwitchHasAuthority
      (:Authority
        _)
      (:Remote
        _))
    (Pawn|UnPossess)))

(event Input|KeyboardEvents|M
  (params (Key :type Key%20Structure :default "None"))
  (:Pressed
    (Networking|SwitchHasAuthority
      (:Authority
        (CallFunction|ServerPossess))
      (:Remote
        (CallFunction|ForClientPossess)))))

(fn ConstructionScript)

(fn OnRepCubePawn)

(fn OnRepClientCubePawn)