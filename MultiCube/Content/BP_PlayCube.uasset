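; BP_PlayCube is a Blueprint that attempts online session setup on BeginPlay, branching on network authority.
; With authority it starts a session search, then calls a session node without waiting for results and prints on success.
; Remote instances start the same search, then immediately try joining an empty session result rather than a found one, printing success or failure.
; The construction script and RepNotify function are empty.
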(event EventBeginPlay
  (bind _returnvalue (Game|GetPlayerController 0))
  (bind _returnvalue_2 (Game|GetPlayerController 0))
  (Networking|SwitchHasAuthority
    (:Authority
      (|FindSessions _returnvalue_2 0 false
        (:then
          (|Session _returnvalue_2 0 false
            (:OnSuccess
              (Development|PrintString "On Session"))))))
    (:Remote
      (|FindSessions _returnvalue 0 false
        (:then
          (|JoinSession _returnvalue (Utilities|Struct|MakeBlueprintSessionResult)
            (:OnSuccess
              (Development|PrintString "Yes"))
            (:OnFailure
              (Development|PrintString "No"))))))))

(fn ConstructionScript)

(fn OnRepNewVar0)